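; BP_Character is a playable character Blueprint with movement, jumping and basic health.
; Movement input follows control yaw, scaled by a Speed variable that rises while Tab is held.
; AnyDamage triggers a brief material flash, subtracts Health and only prints on death; the flash restores a different material slot than it changes.
; GameOver is a stub that only casts to BP_MyGameMode1, and Damaged just prints.
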(event Custom|Damaged
  (Development|PrintString "Damaged"))

(event Custom|DamagedBody
  (bind _mesh (Variables|Character|GetMesh))
  (Rendering|Material|SetMaterial _mesh 0 "/Game/Materials/DamagedMaterial.DamagedMaterial")
  (Utilities|FlowControl|Delay 0.2)
  (Rendering|Material|SetMaterial _mesh 2 "/Game/Materials/T_Liz_Body_Mat.T_Liz_Body_Mat"))

(event Custom|GameOver
  (params (Clear :type Boolean))
  (Utilities|Casting|CastToBP_MyGameMode1 (Game|GetGameMode)))

(event EventBeginPlay)

(event Collision|EventActorBeginOverlap
  (params (OtherActor :type Actor%20Object%20Reference)))

(event EventTick
  (params (DeltaSeconds :type Float%20%28single-precision%29)))

(event Game|Damage|EventAnyDamage
  (params (Damage :type Float%20%28single-precision%29) (DamageType :type Damage%20Type%20Object%20Reference) (InstigatedBy :type Controller%20Object%20Reference) (DamageCauser :type Actor%20Object%20Reference))
  (CallFunction|DamagedBody)
  (bind _output_get (Variables|Default|SetHealth (- (Variables|Default|GetHealth) Damage)))
  (Development|PrintString (Utilities|String|ToString(Float) _output_get))
  (Development|PrintString "HP")
  (if (<= _output_get 0.0)
    (Development|PrintString "Dead")))

(event Input|ActionEvents|InputActionJump
  (params (Key :type Key%20Structure :default "None"))
  ;[1 1 1] 캐릭터 점프
  (:Pressed
    (Character|Jump)))

(event Input|AxisEvents|InputAxisMoveForward
  (params (AxisValue :type Float%20%28single-precision%29))
  ;[1 1 1] 캐릭터 이동
  (Pawn|Input|AddMovementInput (Math|Vector|GetForwardVector (Math|Rotator|MakeRotator 0.0 0.0 (.Yaw (Math|Rotator|BreakRotator (Pawn|GetControlRotation :!class /Script/Engine.Pawn))))) (* AxisValue (Variables|Default|GetSpeed)) false))

(event Input|AxisEvents|InputAxisMoveRight
  (params (AxisValue :type Float%20%28single-precision%29))
  ;[1 1 1] 캐릭터 이동
  (Pawn|Input|AddMovementInput (Math|Vector|GetRightVector (Math|Rotator|MakeRotator 0.0 0.0 (.Yaw (Math|Rotator|BreakRotator (Pawn|GetControlRotation :!class /Script/Engine.Pawn))))) (* AxisValue (Variables|Default|GetSpeed)) false))

(event Input|KeyboardEvents|Tab
  (params (Key :type Key%20Structure :default "None"))
  ;[1 1 1] 캐릭터 이동
  (:Pressed
    (Variables|Default|SetSpeed 0.7))
  (:Released
    (Variables|Default|SetSpeed 0.5)))

(fn ConstructionScript)