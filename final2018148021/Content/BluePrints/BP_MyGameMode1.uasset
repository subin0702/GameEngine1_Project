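; BP_MyGameMode1 is a game mode that tracks score and progress through the BP_Light actors in the level.
; Every Tick it recounts all BP_Light actors and sets Exploding to true when that count equals PassedLights, which this file never updates.
; AddScore increments TotalScore by one, independently of the light check.
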(event EventBeginPlay)

(event EventTick
  (params (DeltaSeconds :type Float%20%28single-precision%29))
  (bind _outactors (Actor|GetAllActorsOfClass "/Game/BluePrints/BP_Light.BP_Light_C"))
  (bind _output_get (Variables|Default|SetNumberOfLights (Utilities|Array|Length _outactors)))
  (if (== _output_get (Variables|Default|GetPassedLights))
    (Variables|Default|SetExploding true)))

(fn ConstructionScript)

(fn AddScore
  (Variables|Default|SetTotalScore (+ (Variables|Default|GetTotalScore) 1)))